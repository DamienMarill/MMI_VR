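; BP_MasterInfo runs a five-level VR tracing puzzle where a laser goes from each drawing's InBall to its OutBall, printing "gagné" after the last.
; BeginPlay hides and parks levels 2-5, saving their positions to restore as each level is reached.
; Each Tick, while the second motion controller grips, a hand sphere trace sets IsInPath, advances levels and places the laser.
; Leaving the drawing resets the path, except on the last level.
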(event EventBeginPlay
  (bind _posblueprint (Variables|Default|GetposBlueprint))
  ;[1 1 1] cacher LVL 2
  (bind _outactors (Actor|GetAllActorsOfClass "/Game/salle_infographie/Blueprint/BP_dessin_lvl2.BP_dessin_lvl2_C"))
  (bind _asbp_dessin_lvl_2 (Utilities|Casting|CastToBP_dessin_lvl2 (Utilities|Array|Get(acopy) _outactors)))
  (Rendering|SetActorHiddenInGame _asbp_dessin_lvl_2 true)
  (Utilities|Array|Add _posblueprint (Transformation|GetActorLocation _asbp_dessin_lvl_2))
  (Transformation|SetActorLocation _asbp_dessin_lvl_2 "-150.000000, 0, 0" false false)
  ;[1 1 1] cacher LVL 3
  (bind _outactors_2 (Actor|GetAllActorsOfClass "/Game/salle_infographie/Blueprint/BP_dessin_lvl3.BP_dessin_lvl3_C"))
  (bind _asbp_dessin_lvl_3 (Utilities|Casting|CastToBP_dessin_lvl3 (Utilities|Array|Get(acopy) _outactors_2)))
  (Rendering|SetActorHiddenInGame _asbp_dessin_lvl_3 true)
  (Utilities|Array|Add _posblueprint (Transformation|GetActorLocation _asbp_dessin_lvl_3))
  (Transformation|SetActorLocation _asbp_dessin_lvl_3 "-150.000000, 0, 0" false false)
  ;[1 1 1] cacher LVL 4
  (bind _outactors_3 (Actor|GetAllActorsOfClass "/Game/salle_infographie/Blueprint/BP_dessin_lvl4.BP_dessin_lvl4_C"))
  (bind _asbp_dessin_lvl_4 (Utilities|Casting|CastToBP_dessin_lvl4 (Utilities|Array|Get(acopy) _outactors_3)))
  (Rendering|SetActorHiddenInGame _asbp_dessin_lvl_4 true)
  (Utilities|Array|Add _posblueprint (Transformation|GetActorLocation _asbp_dessin_lvl_4))
  (Transformation|SetActorLocation _asbp_dessin_lvl_4 "-150.000000, 0, 0" false false)
  ;[1 1 1] cacher LVL 5
  (bind _outactors_4 (Actor|GetAllActorsOfClass "/Game/salle_infographie/Blueprint/BP_dessin_lvl5.BP_dessin_lvl5_C"))
  (bind _asbp_dessin_lvl_5 (Utilities|Casting|CastToBP_dessin_lvl5 (Utilities|Array|Get(acopy) _outactors_4)))
  (Rendering|SetActorHiddenInGame _asbp_dessin_lvl_5 true)
  (Utilities|Array|Add _posblueprint (Transformation|GetActorLocation _asbp_dessin_lvl_5))
  (Transformation|SetActorLocation _asbp_dessin_lvl_5 "-150.000000, 0, 0" false false))

(event Collision|EventActorBeginOverlap
  (params (OtherActor :type Actor%20Object%20Reference)))

(event EventTick
  (params (DeltaSeconds :type Float%20%28single-precision%29))
  (bind _scene (Variables|Default|GetScene))
  (bind _p_ky_stabshot_b (Variables|Default|GetP_ky_stabShot_B))
  (bind _p_ky_stabshot (Variables|Default|GetP_ky_stabShot))
  (bind _posblueprint (Variables|Default|GetposBlueprint))
  (bind _outactors (Actor|GetAllActorsOfClass "/Game/VirtualRealityBP/Blueprints/BP_MotionController.BP_MotionController_C"))
  (bind _asbp_motion_controller (Utilities|Casting|CastToBP_MotionController (Utilities|Array|Get(acopy) _outactors 1)))
  (switch Utilities|FlowControl|Switch|SwitchonGripEnum (Variables|/Game/VirtualRealityBP/Blueprints/BP_MotionController.BP_MotionController_C|GetGripState _asbp_motion_controller)
    (:NewEnumerator0
      (Development|SetHiddeninGame (Variables|Default|GetP_ky_stabShot) true false)
      (Variables|Default|SetisInPath false))
    (:NewEnumerator2
      (bind _outhit (Collision|SphereTraceByChannel (Transformation|GetSocketLocation (Variables|/Game/VirtualRealityBP/Blueprints/BP_MotionController.BP_MotionController_C|GetHandMesh _asbp_motion_controller) "hand_rSocket") (+ (Transformation|GetSocketLocation (Variables|/Game/VirtualRealityBP/Blueprints/BP_MotionController.BP_MotionController_C|GetHandMesh _asbp_motion_controller) "hand_rSocket") (* (Math|Vector|GetForwardVector (Variables|/Game/VirtualRealityBP/Blueprints/BP_MotionController.BP_MotionController_C|GetArcDirection _asbp_motion_controller)) 1e+04)) 5.0 "TraceTypeQuery1" false 0 "None" true "(R=1.000000,G=0.000000,B=0.000000,A=1.000000)" "(R=0.000000,G=1.000000,B=0.000000,A=1.000000)" 1.0))
      (if true
        (Utilities|FlowControl|Sequence
          (:then_0
            (switch int (Variables|Default|Getlvl)
              (:0
                (bind _asbp_dessin_lvl_1 (Utilities|Casting|CastToBP_dessin_lvl1 (.HitActor (Collision|BreakHitResult _outhit)))
                  (:then
                    (if (== (Variables|/Game/salle_infographie/Blueprint/BP_dessin.BP_dessin_C|Getin_ball _asbp_dessin_lvl_1) (.HitComponent (Collision|BreakHitResult _outhit)))
                      (Variables|Default|SetisInPath true :!label _label)
                      (Development|SetHiddeninGame _p_ky_stabshot_b false false)
                      (Development|SetHiddeninGame _p_ky_stabshot true false)
                      (elif (and (== (Variables|/Game/salle_infographie/Blueprint/BP_dessin.BP_dessin_C|Getout_ball _asbp_dessin_lvl_1) (.HitComponent (Collision|BreakHitResult _outhit))) (Variables|Default|GetisInPath))
                        (Utilities|FlowControl|Sequence
                          (:then_0
                            (Variables|Default|SetisInPath false :!label _label_2)
                            (Development|SetHiddeninGame _p_ky_stabshot_b true false)
                            (Development|SetHiddeninGame _p_ky_stabshot false false))
                          (:then_1
                            (Rendering|SetActorHiddenInGame _asbp_dessin_lvl_1 true)
                            (Transformation|SetActorLocation _asbp_dessin_lvl_1 "-150.000000, 0, 0" false false)
                            (bind _output_get (Variables|Default|Setlvl (+ (Variables|Default|Getlvl) 1) :!label _label_3))
                            (switch int _output_get
                              (:1
                                (Rendering|SetActorHiddenInGame (stale EventBeginPlay _asbp_dessin_lvl_2) false)
                                (Transformation|SetActorLocation (stale EventBeginPlay _asbp_dessin_lvl_2) (Utilities|Array|Get(acopy) _posblueprint) false false))
                              (:2
                                (Rendering|SetActorHiddenInGame (stale EventBeginPlay _asbp_dessin_lvl_3) false)
                                (Transformation|SetActorLocation (stale EventBeginPlay _asbp_dessin_lvl_3) (Utilities|Array|Get(acopy) _posblueprint 1) false false))
                              (:3
                                (Rendering|SetActorHiddenInGame (stale EventBeginPlay _asbp_dessin_lvl_4) false)
                                (Transformation|SetActorLocation (stale EventBeginPlay _asbp_dessin_lvl_4) (Utilities|Array|Get(acopy) _posblueprint 2) false false))
                              (:4
                                (Rendering|SetActorHiddenInGame (stale EventBeginPlay _asbp_dessin_lvl_5) false)
                                (Transformation|SetActorLocation (stale EventBeginPlay _asbp_dessin_lvl_5) (Utilities|Array|Get(acopy) _posblueprint 3) false false))
                              (:5
                                (Development|PrintString "gagné" true true "(R=1.000000,G=0.958173,B=0.095608,A=1.000000)" 2e+01))))))))
                  (:CastFailed
                    (goto _label_2))))
              (:1
                (bind _asbp_dessin_lvl_2 (Utilities|Casting|CastToBP_dessin_lvl2 (.HitActor (Collision|BreakHitResult _outhit)))
                  (:then
                    (if (== (Variables|/Game/salle_infographie/Blueprint/BP_dessin.BP_dessin_C|Getin_ball _asbp_dessin_lvl_2) (.HitComponent (Collision|BreakHitResult _outhit)))
                      (goto _label)
                      (elif (and (== (Variables|/Game/salle_infographie/Blueprint/BP_dessin.BP_dessin_C|Getout_ball _asbp_dessin_lvl_2) (.HitComponent (Collision|BreakHitResult _outhit))) (Variables|Default|GetisInPath))
                        (Utilities|FlowControl|Sequence
                          (:then_0
                            (goto _label_2))
                          (:then_1
                            (Rendering|SetActorHiddenInGame _asbp_dessin_lvl_2 true)
                            (Transformation|SetActorLocation _asbp_dessin_lvl_2 "-150.000000, 0, 0" false false)
                            (goto _label_3))))))
                  (:CastFailed
                    (goto _label_2))))
              (:2
                (bind _asbp_dessin_lvl_3 (Utilities|Casting|CastToBP_dessin_lvl3 (.HitActor (Collision|BreakHitResult _outhit)))
                  (:then
                    (if (== (Variables|/Game/salle_infographie/Blueprint/BP_dessin.BP_dessin_C|Getin_ball _asbp_dessin_lvl_3) (.HitComponent (Collision|BreakHitResult _outhit)))
                      (goto _label)
                      (elif (and (== (Variables|/Game/salle_infographie/Blueprint/BP_dessin.BP_dessin_C|Getout_ball _asbp_dessin_lvl_3) (.HitComponent (Collision|BreakHitResult _outhit))) (Variables|Default|GetisInPath))
                        (Utilities|FlowControl|Sequence
                          (:then_0
                            (goto _label_2))
                          (:then_1
                            (Rendering|SetActorHiddenInGame _asbp_dessin_lvl_3 true)
                            (Transformation|SetActorLocation _asbp_dessin_lvl_3 "-150.000000, 0, 0" false false)
                            (goto _label_3))))))
                  (:CastFailed
                    (goto _label_2))))
              (:3
                (bind _asbp_dessin_lvl_4 (Utilities|Casting|CastToBP_dessin_lvl4 (.HitActor (Collision|BreakHitResult _outhit)))
                  (:then
                    (if (== (Variables|/Game/salle_infographie/Blueprint/BP_dessin.BP_dessin_C|Getin_ball _asbp_dessin_lvl_4) (.HitComponent (Collision|BreakHitResult _outhit)))
                      (goto _label)
                      (elif (and (== (Variables|/Game/salle_infographie/Blueprint/BP_dessin.BP_dessin_C|Getout_ball _asbp_dessin_lvl_4) (.HitComponent (Collision|BreakHitResult _outhit))) (Variables|Default|GetisInPath))
                        (Utilities|FlowControl|Sequence
                          (:then_0
                            (goto _label_2))
                          (:then_1
                            (Rendering|SetActorHiddenInGame _asbp_dessin_lvl_4 true)
                            (Transformation|SetActorLocation _asbp_dessin_lvl_4 "-150.000000, 0, 0" false false)
                            (goto _label_3))))))
                  (:CastFailed
                    (goto _label_2))))
              (:4
                (bind _asbp_dessin_lvl_5 (Utilities|Casting|CastToBP_dessin_lvl5 (.HitActor (Collision|BreakHitResult _outhit))))
                (if (== (Variables|/Game/salle_infographie/Blueprint/BP_dessin.BP_dessin_C|Getin_ball _asbp_dessin_lvl_5) (.HitComponent (Collision|BreakHitResult _outhit)))
                  (goto _label)
                  (elif (and (== (Variables|/Game/salle_infographie/Blueprint/BP_dessin.BP_dessin_C|Getout_ball _asbp_dessin_lvl_5) (.HitComponent (Collision|BreakHitResult _outhit))) (Variables|Default|GetisInPath))
                    (Utilities|FlowControl|Sequence
                      (:then_0
                        (goto _label_2))
                      (:then_1
                        (Rendering|SetActorHiddenInGame _asbp_dessin_lvl_5 true)
                        (Transformation|SetActorLocation _asbp_dessin_lvl_5 "-150.000000, 0, 0" false false)
                        (goto _label_3))))))))
          (:then_1
            (if (Variables|Default|GetisInPath)
              (Variables|Default|Seti 1)
              (else
                (Variables|Default|Seti 0)))
            (Transformation|SetWorldLocation _scene (.Location (Collision|BreakHitResult _outhit)) false true)
            (Transformation|SetRelativeScale3D _scene (Math|Vector|MakeVector (/ (.Distance (Collision|BreakHitResult _outhit)) 6e+02) (Utilities|Array|Get(acopy) (Variables|Default|GetCircLaser) (Variables|Default|Geti)) (Utilities|Array|Get(acopy) (Variables|Default|GetCircLaser) (Variables|Default|Geti))))
            (Transformation|SetRelativeRotation _scene (Transformation|GetWorldRotation (Variables|/Game/VirtualRealityBP/Blueprints/BP_MotionController.BP_MotionController_C|GetHandMesh _asbp_motion_controller)) false false)))
        (else
          (goto _label_2))))))

(fn ConstructionScript)