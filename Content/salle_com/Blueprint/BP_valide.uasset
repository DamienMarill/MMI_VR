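; BP_valide is a validation trigger that scores the selection state of BP_obj actors and displays the result.
; When anything begins overlapping its Box, it gathers every BP_obj and compares IsSelect with ASelect, apparently the expected answer.
; Correct selections add a point, while missed or wrong ones subtract one.
; Points are written to a TextRender and never reset here, so repeated overlaps accumulate.
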(event OnComponentBeginOverlap(Box)
  (params (OverlappedComponent :type Primitive%20Component%20Object%20Reference) (OtherActor :type Actor%20Object%20Reference) (OtherComp :type Primitive%20Component%20Object%20Reference) (OtherBodyIndex :type Integer) (bFromSweep :type Boolean) (SweepResult :type Hit%20Result%20Structure%20%28by%20ref%29))
  (bind _outactors (Actor|GetAllActorsOfClass "/Game/salle_com/Blueprint/BP_obj.BP_obj_C"))
  (for _array_element _outactors
    (bind _asbp_obj (Utilities|Casting|CastToBP_obj _array_element))
    (if (Variables|/Game/salle_com/Blueprint/BP_obj.BP_obj_C|GetaSelect _asbp_obj)
      (if (Variables|/Game/salle_com/Blueprint/BP_obj.BP_obj_C|GetisSelect _asbp_obj)
        (Variables|Default|Setpoints (+ (Variables|Default|Getpoints) 1))
        (else
          (Variables|Default|Setpoints (- (Variables|Default|Getpoints) 1) :!label _label)))
      (elif (Variables|/Game/salle_com/Blueprint/BP_obj.BP_obj_C|GetisSelect _asbp_obj)
        (goto _label))))
  (Rendering|Components|TextRender|SetText (Variables|Default|GetTextRender) (Utilities|Text|ToText(Integer) (Variables|Default|Getpoints))))

(event EventBeginPlay)

(event Collision|EventActorBeginOverlap
  (params (OtherActor :type Actor%20Object%20Reference)))

(event EventTick
  (params (DeltaSeconds :type Float%20%28single-precision%29)))

(fn ConstructionScript)