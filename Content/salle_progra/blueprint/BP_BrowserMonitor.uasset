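; Monitor actor that displays a web page through a web browser widget on a 3D widget component.
; On BeginPlay it sends the base URL to the widget through the BPI_WebBrowser interface.
; UpdtScreen appends a parameter and value to the base URL as a query string, updating the browser only when that differs from the current URL.
; Each URL is also printed on screen for debugging.
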(event EventBeginPlay
  (bind _output_get (Variables|Default|SetCurrentURL (Variables|Default|GetBaseURL)))
  (Development|PrintString _output_get true true "(R=0.000000,G=0.660000,B=1.000000,A=1.000000)" 2e+02)
  (bind _asbpi_web_browser (Utilities|Casting|CastToBPI_WebBrowser (UserInterface|GetUserWidgetObject (Variables|Default|Get3DWidget))))
  (Default|UpdURL _asbpi_web_browser _output_get))

(event Collision|EventActorBeginOverlap
  (params (OtherActor :type Actor%20Object%20Reference)))

(event EventTick
  (params (DeltaSeconds :type Float%20%28single-precision%29)))

(fn ConstructionScript)

(fn UpdtScreen
  (params (Param :type Text) (Value :type Text))
  (bind _returnvalue (Utilities|String|ToString(Text) Param))
  (bind _returnvalue_2 (Utilities|String|ToString(Text) Value))
  (bind _baseurl (Variables|Default|GetBaseURL))
  (bind _returnvalue_3 (Utilities|String|Append _baseurl "?" _returnvalue "=" _returnvalue_2))
  (if (Utilities|Enum|NotEqual(Enum) (Variables|Default|GetCurrentURL) _returnvalue_3)
    (Development|PrintString _returnvalue_3 true true "(R=0.000000,G=0.660000,B=1.000000,A=1.000000)" 2e+03)
    (bind _asbpi_web_browser (Utilities|Casting|CastToBPI_WebBrowser (UserInterface|GetUserWidgetObject (Variables|Default|Get3DWidget))))
    (Default|UpdURL _asbpi_web_browser _returnvalue_3)
    (Variables|Default|SetCurrentURL _returnvalue_3)))