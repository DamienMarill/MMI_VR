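; Menu button actor that displays a text value and applies it to the currently selected style attribute when its Box is overlapped.
; On overlap it calls UpdtValue on the first Menu actor found, then turns its own label blue.
; It stores ButtonText in the Menu variable matching CurrentAttr (background color, size, color, left margin or opacity).
; It then passes that attribute and value to the first BP_BrowserMonitor via UpdtScreen.
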(event OnComponentBeginOverlap(Box)
  (params (OverlappedComponent :type Primitive%20Component%20Object%20Reference) (OtherActor :type Actor%20Object%20Reference) (OtherComp :type Primitive%20Component%20Object%20Reference) (OtherBodyIndex :type Integer) (bFromSweep :type Boolean) (SweepResult :type Hit%20Result%20Structure%20%28by%20ref%29))
  (bind _button_text (Variables|Default|GetButton_Text))
  (bind _outactors (Actor|GetAllActorsOfClass "/Game/salle_progra/blueprint/menu/Menu.Menu_C"))
  (bind _asmenu (Utilities|Casting|CastToMenu (Utilities|Array|Get(acopy) _outactors)))
  (Default|UpdtValue _asmenu)
  (Rendering|Components|TextRender|SetTextRenderColor (Variables|Default|GetTextRender) (Math|Color|MakeColor 255 0 0))
  (switch string (Utilities|String|ToString(Text) (Variables|/Game/salle_progra/blueprint/menu/Menu.Menu_C|GetCurrentAttr _asmenu))
    (:bgColor
      (Variables|/Game/salle_progra/blueprint/menu/Menu.Menu_C|SetV_BgColor _asmenu _button_text))
    (:size
      (Variables|/Game/salle_progra/blueprint/menu/Menu.Menu_C|SetV_FontSize _asmenu _button_text))
    (:color
      (Variables|/Game/salle_progra/blueprint/menu/Menu.Menu_C|SetV_Color _asmenu _button_text))
    (:marginLeft
      (Variables|/Game/salle_progra/blueprint/menu/Menu.Menu_C|SetV_MarginLeft _asmenu _button_text))
    (:opacity
      (Variables|/Game/salle_progra/blueprint/menu/Menu.Menu_C|SetV_Opacity _asmenu _button_text)))
  (bind _outactors_2 (Actor|GetAllActorsOfClass "/Game/salle_progra/blueprint/BP_BrowserMonitor.BP_BrowserMonitor_C"))
  (bind _asbp_browser_monitor (Utilities|Casting|CastToBP_BrowserMonitor (Utilities|Array|Get(acopy) _outactors_2)))
  (Default|UpdtScreen _asbp_browser_monitor (Variables|/Game/salle_progra/blueprint/menu/Menu.Menu_C|GetCurrentAttr _asmenu) _button_text))

(event EventBeginPlay
  (|CallParentFunction)
  (Rendering|Components|TextRender|SetText (Variables|Default|GetTextRender) (Variables|Default|GetButton_Text)))

(event Collision|EventActorBeginOverlap
  (params (OtherActor :type Actor%20Object%20Reference))
  (|CallParentFunction OtherActor) ; This node is disabled and will not be called.\nDrag off pins to build functionality.
)

(event EventTick
  (params (DeltaSeconds :type Float%20%28single-precision%29))
  (|CallParentFunction DeltaSeconds) ; This node is disabled and will not be called.\nDrag off pins to build functionality.
)

(fn ConstructionScript
  (|CallParentFunction))