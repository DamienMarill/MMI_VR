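; BP_ButtonAttr is an in-world menu button actor that selects an attribute when something overlaps its box.
; The construction script sets its text render label from ButtonText.
; On overlap it finds the first Menu actor and, if that attribute is not already current, passes it the attribute name and value list, calls UpdtAttr and turns its own label blue.
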(event OnComponentBeginOverlap(Box)
  (params (OverlappedComponent :type Primitive%20Component%20Object%20Reference) (OtherActor :type Actor%20Object%20Reference) (OtherComp :type Primitive%20Component%20Object%20Reference) (OtherBodyIndex :type Integer) (bFromSweep :type Boolean) (SweepResult :type Hit%20Result%20Structure%20%28by%20ref%29))
  (bind _attrname (Variables|Default|GetAttrName))
  (Development|PrintString (Utilities|String|ToString(Text) (Variables|Default|GetButton_Text)))
  (bind _outactors (Actor|GetAllActorsOfClass "/Game/salle_progra/blueprint/menu/Menu.Menu_C"))
  (bind _asmenu (Utilities|Casting|CastToMenu (Utilities|Array|Get(acopy) _outactors)))
  (if (Utilities|Enum|NotEqual(Enum) (Variables|/Game/salle_progra/blueprint/menu/Menu.Menu_C|GetCurrentAttr _asmenu) _attrname)
    (Variables|/Game/salle_progra/blueprint/menu/Menu.Menu_C|SetCurrentAttr _asmenu _attrname)
    (Variables|/Game/salle_progra/blueprint/menu/Menu.Menu_C|SetCurrentValue _asmenu (Variables|Default|GetvaluesLst))
    (Default|UpdtAttr _asmenu)
    (Rendering|Components|TextRender|SetTextRenderColor (Variables|Default|GetTextRender) (Math|Color|MakeColor 255 0 0))))

(event EventBeginPlay
  (|CallParentFunction) ; This node is disabled and will not be called.\nDrag off pins to build functionality.
)

(event Collision|EventActorBeginOverlap
  (params (OtherActor :type Actor%20Object%20Reference))
  (|CallParentFunction OtherActor) ; This node is disabled and will not be called.\nDrag off pins to build functionality.
)

(event EventTick
  (params (DeltaSeconds :type Float%20%28single-precision%29))
  (|CallParentFunction DeltaSeconds) ; This node is disabled and will not be called.\nDrag off pins to build functionality.
)

(fn ConstructionScript
  (|CallParentFunction)
  (Rendering|Components|TextRender|SetText (Variables|Default|GetTextRender) (Variables|Default|GetButton_Text)))