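; Menu actor for choosing style attributes (background color, size, color, left margin, opacity) and their values through in-world text buttons.
; UpdtAttr resets all attribute button colors, prints the current attribute, then fills each value button from CurrentValue by array index.
; It switches on the attribute name to highlight the value matching that attribute's stored variable in blue.
; UpdtValue only resets value button colors; the event graph is empty.
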(event EventBeginPlay)

(event Collision|EventActorBeginOverlap
  (params (OtherActor :type Actor%20Object%20Reference)))

(event EventTick
  (params (DeltaSeconds :type Float%20%28single-precision%29)))

(fn ConstructionScript)

(fn UpdtAttr
  (bind _outactors (Actor|GetAllActorsOfClass "/Game/salle_progra/blueprint/menu/BP_ButtonAttr.BP_ButtonAttr_C"))
  (for _array_element _outactors
    (Rendering|Components|TextRender|SetTextRenderColor (Variables|/Game/salle_progra/blueprint/menu/BP_ButtonParent.BP_ButtonParent_C|GetTextRender _array_element) (Math|Color|MakeColor 0 0 0)))
  (Development|PrintString (Utilities|String|ToString(Text) (Variables|Default|GetCurrentAttr)))
  (bind _outactors_2 (Actor|GetAllActorsOfClass "/Game/salle_progra/blueprint/menu/BP_ButtonValue.BP_ButtonValue_C"))
  (for (_array_element_2 _array_index) _outactors_2
    (Variables|/Game/salle_progra/blueprint/menu/BP_ButtonValue.BP_ButtonValue_C|SetButton_Text _array_element_2 (Utilities|Array|Get(acopy) (Variables|Default|GetCurrentValue) _array_index))
    (Rendering|Components|TextRender|SetText (Variables|/Game/salle_progra/blueprint/menu/BP_ButtonParent.BP_ButtonParent_C|GetTextRender _array_element_2) (Utilities|Array|Get(acopy) (Variables|Default|GetCurrentValue) _array_index))
    (switch string (Utilities|String|ToString(Text) (Variables|Default|GetCurrentAttr))
      (:bgColor
        (if (Utilities|Enum|Equal(Enum) (Variables|Default|GetV_BgColor) (Utilities|Array|Get(acopy) (Variables|Default|GetCurrentValue) _array_index))
          (Rendering|Components|TextRender|SetTextRenderColor (Variables|/Game/salle_progra/blueprint/menu/BP_ButtonParent.BP_ButtonParent_C|GetTextRender _array_element_2) (Math|Color|MakeColor 255 0 0) :!label _label)
          (else
            (Rendering|Components|TextRender|SetTextRenderColor (Variables|/Game/salle_progra/blueprint/menu/BP_ButtonParent.BP_ButtonParent_C|GetTextRender _array_element_2) (Math|Color|MakeColor 0 0 0) :!label _label_2))))
      (:size
        (if (Utilities|Enum|Equal(Enum) (Variables|Default|GetV_FontSize) (Utilities|Array|Get(acopy) (Variables|Default|GetCurrentValue) _array_index))
          (goto _label)
          (else
            (goto _label_2))))
      (:color
        (if (Utilities|Enum|Equal(Enum) (Variables|Default|GetV_Color) (Utilities|Array|Get(acopy) (Variables|Default|GetCurrentValue) _array_index))
          (goto _label)
          (else
            (goto _label_2))))
      (:marginLeft
        (if (Utilities|Enum|Equal(Enum) (Variables|Default|GetV_MarginLeft) (Utilities|Array|Get(acopy) (Variables|Default|GetCurrentValue) _array_index))
          (goto _label)
          (else
            (goto _label_2))))
      (:opacity
        (if (Utilities|Enum|Equal(Enum) (Variables|Default|GetV_Opacity) (Utilities|Array|Get(acopy) (Variables|Default|GetCurrentValue) _array_index))
          (goto _label)
          (else
            (goto _label_2)))))))

(fn UpdtValue
  (bind _outactors (Actor|GetAllActorsOfClass "/Game/salle_progra/blueprint/menu/BP_ButtonValue.BP_ButtonValue_C"))
  (for _array_element _outactors
    (Rendering|Components|TextRender|SetTextRenderColor (Variables|/Game/salle_progra/blueprint/menu/BP_ButtonParent.BP_ButtonParent_C|GetTextRender _array_element) (Math|Color|MakeColor 0 0 0))))